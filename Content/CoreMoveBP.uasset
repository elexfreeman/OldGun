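; CoreMoveBP is a projectile actor (the "core") that is launched by physics and explodes after a set lifetime.
; OnFire enables physics simulation on the mesh, applies the direction vector as an impulse and starts a one-shot lifetime timer.
; When the timer fires, it hides the mesh and PExplosion component, spawns ExplodeBP at the mesh's location and destroys itself after a short delay.
; Detonation is purely timed, with no active collision or overlap logic.
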(event Custom|OnFire
  (params (direction :type Vector))
  ;[1 1 1] Включаем физику и добавляем импульс
  (Physics|SetSimulatePhysics (Variables|Default|GetStaticMesh) true)
  (Physics|AddImpulse (Variables|Default|GetStaticMesh) direction "None" false)
  ;[1 1 1] По таймауту спавним взрыв и дестроимся
  (Utilities|Time|SetTimerbyEvent (delegate Custom|OnDestroyCore) (Variables|Default|GetnCoreLifeTime)))

(event Custom|OnDestroyCore
  ;[1 1 1] По таймауту спавним взрыв и дестроимся
  (Rendering|SetVisibility (Variables|Default|GetP_Explosion) false false)
  (Rendering|SetVisibility (Variables|Default|GetStaticMesh) false false)
  ;;[1 1 1] Спавним взрыв
  (Game|SpawnActorfromClass "/OldGun/ExplodeBP.ExplodeBP_C" (Math|Conversions|ToTransform(Vector) (Transformation|GetWorldLocation (Variables|Default|GetStaticMesh))) "Undefined" 0 0)
  (Utilities|FlowControl|Delay 0.5)
  (Actor|DestroyActor))

(event EventBeginPlay)

(event Collision|EventActorBeginOverlap
  (params (OtherActor :type Actor%20Object%20Reference)))

(event EventTick
  (params (DeltaSeconds :type Float%20%28single-precision%29)))

(fn ConstructionScript)

(fn FInit)