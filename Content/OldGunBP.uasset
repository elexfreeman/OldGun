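; OldGunBP is an old gun actor that fires a CoreMoveBP projectile after a short fuse-like delay.
; Firing calls an event dispatcher, shows the PSparks effect and starts a one-shot timer.
; When the timer ends, it calls a done dispatcher, hides the sparks and spawns the projectile at CoreSpawnPoint.
; It passes the projectile a Force-scaled direction from Gun1 to the spawn point, also printed for debugging.
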(event Custom|onFire
  (Default|CallOnFireEvent)
  (Rendering|SetVisibility (Variables|Default|GetP_Sparks) true false)
  (Utilities|Time|SetTimerbyEvent (delegate Custom|onFireDone) 1.0))

(event Custom|onFireDone
  (bind _corespawnpoint (Variables|Default|GetCoreSpawnPoint))
  (bind _gun1 (Variables|Default|GetGun1))
  (bind _force (Variables|AA|GetForce))
  (bind _returnvalue (Transformation|GetWorldLocation _corespawnpoint))
  (bind _returnvalue_2 (Transformation|GetWorldLocation _gun1))
  (bind _returnvalue_3 (Math|Vector|GetUnitDirection(Vector) _returnvalue_2 _returnvalue))
  (bind _returnvalue_4 (* _returnvalue_3 _force))
  (Default|CallOnFireDoneEvent)
  (Rendering|SetVisibility (Variables|Default|GetP_Sparks) false false)
  (bind _returnvalue_5 (Game|SpawnActorfromClass "/OldGun/CoreMoveBP.CoreMoveBP_C" (Transformation|GetWorldTransform (Variables|Default|GetCoreSpawnPoint)) "Undefined" 0 0))
  (Default|OnFire _returnvalue_5 _returnvalue_4)
  (Development|PrintString (Utilities|String|ToString(Vector) _returnvalue_4)))

(event EventBeginPlay)

(event Collision|EventActorBeginOverlap
  (params (OtherActor :type Actor%20Object%20Reference)))

(event EventTick
  (params (DeltaSeconds :type Float%20%28single-precision%29)))

(fn ConstructionScript)